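; Player pawn that rolls a static mesh by physics torque and can restart the current level.
; MoveForward and MoveRight axis inputs feed a single AddTorqueInRadians call as scaled acceleration change, with the X torque negated.
; BeginPlay fades the camera in from black.
; RestartLevel input reopens the current level once through a DoOnce macro, whose fade-out and delay step is disconnected.
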(event `InputAction|RestartLevel`
  (params (Key :type "Key Structure"))
  ;[1 1 1] Restart level
  (:`Pressed`
    (`self.LevelRestart`)))

(event `self.ReceiveBeginPlay`
  (`PlayerCameraManager.StartCameraFade` (`GameplayStatics.GetPlayerCameraManager` 0) 1.0 0.0 1.0 (struct :`A` 1.0) false false))

(event `InputAxis|MoveForward`
  (params (AxisValue :type "Float (single-precision)"))
  ;[1 1 1] Adjusted these values from the original CrystalCavern demo
  (`PrimitiveComponent.AddTorqueInRadians` (`self.StaticMesh`) (`KismetMathLibrary.MakeVector` (* (* (stale `InputAxis|MoveRight` AxisValue) (`self.AccelerationMultiplier`)) -1.0) (* AxisValue (`self.AccelerationMultiplier`))) "None" true :!label _label))

(event `InputAxis|MoveRight`
  (params (AxisValue :type "Float (single-precision)"))
  ;[1 1 1] Adjusted these values from the original CrystalCavern demo
  (goto _label))

(fn `CameraFade`
  (returns (ReturnValue :type "Float (double-precision)"))
  (`PlayerCameraManager.StartCameraFade` (`GameplayStatics.GetPlayerCameraManager` 0) 0.0 1.0 1.0 (struct :`A` 1.0) false true)
  (return 1.0))

(fn `RestartLevel`
  (bind _returnvalue (`GameplayStatics.GetCurrentLevelName` true))
  (`GameplayStatics.OpenLevel` (`KismetStringLibrary.Conv_StringToName` _returnvalue)))

(fn `UserConstructionScript`)