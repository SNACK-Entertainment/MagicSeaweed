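; Spline connector tool that builds a mesh along a spline whose ends can attach to points on two other actors.
; Construction zeroes the actor transform, so world attachment positions work as local spline coordinates, then fetches points through BPI_SplineConnectorToolInterface.
; UpdateSpline snaps non-manual ends to their chosen point's location, up vector and scaled forward tangent.
; It then adds a collidable SplineMeshComponent per segment, with dampened roll.
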(event `UpdateSpline`
  (bind _rolldampening (`self.RollDampening`))
  (bind (_splinestart_manualeditpoint _splinestart_connectingactor _splinestart_connectingpoint _splinestart_tangentstrength _splinestart_listofpoints) (break `/Game/Splinetools/Blueprints/STRUCT_SplineSettings` (`self.SplineStart`)))
  (bind _spline (`self.Spline`))
  (bind _spline_2 (`self.Spline`))
  (bind (_splineend_manualeditpoint _splineend_connectingactor _splineend_connectingpoint _splineend_tangentstrength _splineend_listofpoints) (break `/Game/Splinetools/Blueprints/STRUCT_SplineSettings` (`self.SplineEnd`)))
  (bind _spline_3 (`self.Spline`))
  (bind _output (`|GetArrayItem` _splinestart_listofpoints _splinestart_connectingpoint))
  (bind _output_2 (`|GetArrayItem` _splineend_listofpoints _splineend_connectingpoint))
  (bind _returnvalue (- (`SplineComponent.GetNumberOfSplinePoints` _spline_3) 1))
  (bind _returnvalue_2 (`SceneComponent.K2_GetComponentRotation` _output))
  (bind _returnvalue_3 (`SceneComponent.K2_GetComponentRotation` _output_2))
  (`|ExecutionSequence`
    (:`then_0`
      (`self.UpdateConnection`))
    (:`then_1`
      (if (not _splinestart_manualeditpoint)
        (`SplineComponent.SetLocationAtSplinePoint` _spline_2 0 (`SceneComponent.K2_GetComponentLocation` _output) "Local" false)
        (`SplineComponent.SetUpVectorAtSplinePoint` _spline_2 0 (`KismetMathLibrary.GetUpVector` _returnvalue_2) "Local" false)
        (`SplineComponent.SetTangentAtSplinePoint` _spline_2 0 (* (`KismetMathLibrary.GetForwardVector` _returnvalue_2) _splinestart_tangentstrength) "Local" true)))
    (:`then_2`
      (if (not _splineend_manualeditpoint)
        (`SplineComponent.SetLocationAtSplinePoint` _spline_3 _returnvalue (`SceneComponent.K2_GetComponentLocation` _output_2) "Local" false)
        (`SplineComponent.SetUpVectorAtSplinePoint` _spline_3 _returnvalue (`KismetMathLibrary.GetUpVector` _returnvalue_3) "Local" false)
        (`SplineComponent.SetTangentAtSplinePoint` _spline_3 _returnvalue (* (`KismetMathLibrary.GetForwardVector` _returnvalue_3) (* _splineend_tangentstrength -1.0)) "Local" true)))
    (:`then_3`
      (`ActorComponent.K2_DestroyComponent` (`self.SplineMesh`)))
    (:`then_4`
      (for _index (range (+ (- (`SplineComponent.GetNumberOfSplinePoints` _spline) 2) 1))
        (bind _returnvalue_4 (`AddComponent|NODE_AddSplineMeshComponent-1`))
        (`SplineMeshComponent.SetForwardAxis` _returnvalue_4 (`self.MeshForwardAxis`) false)
        (`StaticMeshComponent.SetStaticMesh` _returnvalue_4 (`self.Mesh`))
        (bind (_location _tangent) (`SplineComponent.GetLocationAndTangentAtSplinePoint` _spline _index "Local"))
        (bind _returnvalue_5 (+ _index 1))
        (bind (_location_2 _tangent_2) (`SplineComponent.GetLocationAndTangentAtSplinePoint` _spline _returnvalue_5 "Local"))
        (`SplineMeshComponent.SetStartAndEnd` _returnvalue_4 _location _tangent _location_2 _tangent_2 false)
        (`SplineMeshComponent.SetStartRoll` _returnvalue_4 (/ (`SplineComponent.GetRollAtSplinePoint` _spline _index "Local") _rolldampening) false)
        (`SplineMeshComponent.SetEndRoll` _returnvalue_4 (/ (`SplineComponent.GetRollAtSplinePoint` _spline _returnvalue_5 "Local") _rolldampening) true)
        (`PrimitiveComponent.SetCollisionEnabled` _returnvalue_4 "QueryAndPhysics")
        (set `self.SplineMesh` _returnvalue_4)))))

(event `UpdateConnection`
  (bind (_splinestart_manualeditpoint _splinestart_connectingactor _splinestart_connectingpoint _splinestart_tangentstrength) (break `/Game/Splinetools/Blueprints/STRUCT_SplineSettings` (`self.SplineStart`)))
  (bind (_splineend_manualeditpoint _splineend_connectingactor _splineend_connectingpoint _splineend_tangentstrength) (break `/Game/Splinetools/Blueprints/STRUCT_SplineSettings` (`self.SplineEnd`)))
  (`|ExecutionSequence`
    (:`then_0`
      (if (`KismetSystemLibrary.DoesImplementInterface` _splinestart_connectingactor "/Game/Splinetools/Blueprints/BPI_SplineConnectorToolInterface.BPI_SplineConnectorToolInterface_C")
        (bind _points (message `/Game/Splinetools/Blueprints/BPI_SplineConnectorToolInterface.GetSplineAttachmentPoints` _splinestart_connectingactor))
        (set `self.SplineStart` (make `/Game/Splinetools/Blueprints/STRUCT_SplineSettings` _splinestart_manualeditpoint _splinestart_connectingactor _splinestart_connectingpoint _splinestart_tangentstrength _points))
        (elif (not _splinestart_manualeditpoint)
          (`KismetSystemLibrary.PrintString` "SPLINE INTERFACE MISSING" true true (struct :`R` 1.0 :`A` 1.0)))))
    (:`then_1`
      (if (`KismetSystemLibrary.DoesImplementInterface` _splineend_connectingactor "/Game/Splinetools/Blueprints/BPI_SplineConnectorToolInterface.BPI_SplineConnectorToolInterface_C")
        (bind _points_2 (message `/Game/Splinetools/Blueprints/BPI_SplineConnectorToolInterface.GetSplineAttachmentPoints` _splineend_connectingactor))
        (set `self.SplineEnd` (make `/Game/Splinetools/Blueprints/STRUCT_SplineSettings` _splineend_manualeditpoint _splineend_connectingactor _splineend_connectingpoint _splineend_tangentstrength _points_2))
        (elif (not _splineend_manualeditpoint)
          (`KismetSystemLibrary.PrintString` "SPLINE INTERFACE MISSING" true true (struct :`R` 1.0 :`A` 1.0)))))))

(fn `UserConstructionScript`
  (`|ExecutionSequence`
    (:`then_0`
      (`self.K2_SetActorLocationAndRotation` (0.0 0.0 0.0)))
    (:`then_1`
      (`self.UpdateConnection`))
    (:`then_3`
      (if (`self.Update`)
        _
        (else
          _))
      (`self.UpdateSpline`)
      (set `self.Update` false))))