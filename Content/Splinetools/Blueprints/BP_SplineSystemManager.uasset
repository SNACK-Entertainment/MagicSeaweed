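; BP_SplineSystemManager is an editor-side manager that batch-updates BP_SplineComponent actors in the level.
; Its construction script treats self-resetting booleans as buttons, run in sequence.
; GetSplineBPs caches every spline actor, and UpdateConnections copies RotationDamping to each one's RollDampening, then chains into UpdateAllSplines.
; UpdateAllSplines calls UpdateSpline on each cached actor; the event graph does nothing at runtime.
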(fn `UserConstructionScript`
  (`|ExecutionSequence`
    (:`then_0`
      (if (`self.GetSplineBPs`)
        (bind _outactors (`GameplayStatics.GetAllActorsOfClass` "/Game/Splinetools/Blueprints/BP_SplineComponent.BP_SplineComponent_C"))
        (set `self.SplineBPs` _outactors)
        (set `self.GetSplineBPs` false)))
    (:`then_1`
      (if (`self.UpdateConnections`)
        (for _array_element (`self.SplineBPs`)
          (set `/Game/Splinetools/Blueprints/BP_SplineComponent.RollDampening` (`self.RotationDamping`) _array_element))
        (set `self.UpdateAllSplines` true)
        (set `self.UpdateConnections` false)))
    (:`then_2`
      (if (`self.UpdateAllSplines`)
        (for _array_element_2 (`self.SplineBPs`)
          (`/Game/Splinetools/Blueprints/BP_SplineComponent.UpdateSpline` _array_element_2))
        (set `self.UpdateAllSplines` false)))))